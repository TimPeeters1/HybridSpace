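; Blueprint function library that plays haptic feedback on a VR player's hand.
; PlayFeedbackOnHand branches on feedback type (Burst or Shake) and intensity (Low or High) to select one of four haptic effect assets.
; It plays the chosen effect on the given hand through the supplied PlayerController.
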(fn PlayFeedbackonHand
  (params (Hand :type EControllerHand%20Enum :default "Left") (Type :type EFeedbackType%20Enum :default "NewEnumerator0") (Intensity :type EFeedbackIntensity%20Enum :default "NewEnumerator0") (PlayerController :type Player%20Controller%20Object%20Reference))
  (switch Utilities|FlowControl|Switch|SwitchonEFeedbackType Type
    (:NewEnumerator0
      (switch Utilities|FlowControl|Switch|SwitchonEFeedbackIntensity Intensity
        (:NewEnumerator0
          (Class|PlayerController|PlayHapticEffect PlayerController "/Game/VR_Interactables/VR_World_Interaction/Blueprints/FeedbackEffects/LowIntensityBurst.LowIntensityBurst" Hand (LocalVariables|GetScale) false))
        (:NewEnumerator1
          (Class|PlayerController|PlayHapticEffect PlayerController "/Game/VR_Interactables/VR_World_Interaction/Blueprints/FeedbackEffects/HighIntensityBurst.HighIntensityBurst" Hand (LocalVariables|GetScale) false))))
    (:NewEnumerator1
      (switch Utilities|FlowControl|Switch|SwitchonEFeedbackIntensity Intensity
        (:NewEnumerator0
          (Class|PlayerController|PlayHapticEffect PlayerController "/Game/VR_Interactables/VR_World_Interaction/Blueprints/FeedbackEffects/LowIntensityShake.LowIntensityShake" Hand (LocalVariables|GetScale) false))
        (:NewEnumerator1
          (Class|PlayerController|PlayHapticEffect PlayerController "/Game/VR_Interactables/VR_World_Interaction/Blueprints/FeedbackEffects/HighIntensityShake.HighIntensityShake" Hand (LocalVariables|GetScale) false))))))