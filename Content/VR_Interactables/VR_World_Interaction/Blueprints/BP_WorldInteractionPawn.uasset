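; VR pawn that lets the player grab, drag, use and point at world objects with both motion controllers.
; On BeginPlay it sets floor tracking, binds a world interactor component to each hand sphere, and gives each hand a trace interactor with a spawned visualiser and widget interaction.
; Pickup inputs drive both pickup and drag, triggers drive use, and thumbstick presses toggle the traces on and off while held.
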(event EventBeginPlay
  ;[1 1 1] Setup Trace Interactor
  (bind _returnvalue (Game|SpawnActorfromClass "/Game/VR_Interactables/VR_Trace_Interaction/Blueprints/BP_TraceVisualiser.BP_TraceVisualiser_C" (Math|Transform|MakeTransform "0, 0, 0") "Undefined" 0 1.0 "8.000000,0.800000,0.800000" 0))
  (Default|Setup (Variables|Default|GetBP_TraceInteractor_L) _returnvalue self "NewEnumerator2" true (Variables|Default|GetWidgetInteraction))
  (bind _returnvalue_2 (Game|SpawnActorfromClass "/Game/VR_Interactables/VR_Trace_Interaction/Blueprints/BP_TraceVisualiser.BP_TraceVisualiser_C" (Math|Transform|MakeTransform "0, 0, 0") "Undefined" 0 1.0 "8.000000,0.800000,0.800000" 0))
  (Default|Setup (Variables|Default|GetBP_TraceInteractor_R) _returnvalue_2 self "NewEnumerator2" true (Variables|Default|GetWidgetInteraction))
  ;[1 1 1] Setup World Interactor
  (Default|Setup (Variables|Default|GetBPC_WorldInteractor_L) (Variables|Default|GetL_Hand_Sphere))
  (Default|Setup (Variables|Default|GetBPC_WorldInteractor_R) (Variables|Default|GetR_Hand_Sphere))
  ;[1 1 1] Set Floor Level
  (Class|HeadMountedDisplayFunctionLibrary|SetTrackingOrigin "Floor"))

(event Input|ActionEvents|InputActionPickupLeft
  (params (Key :type Key%20Structure :default "None"))
  (bind _bpc_worldinteractor_l (Variables|Default|GetBPC_WorldInteractor_L))
  ;[1 1 1] Pickup
  (:Pressed
    (Default|PickupPressed _bpc_worldinteractor_l)
    (Default|DragStart _bpc_worldinteractor_l))
  (:Released
    (Default|PickupReleased _bpc_worldinteractor_l)
    (Default|DragStop _bpc_worldinteractor_l)))

(event Input|ActionEvents|InputActionPickupRight
  (params (Key :type Key%20Structure :default "None"))
  (bind _bpc_worldinteractor_r (Variables|Default|GetBPC_WorldInteractor_R))
  ;[1 1 1] Pickup
  (:Pressed
    (Default|PickupPressed _bpc_worldinteractor_r)
    (Default|DragStart _bpc_worldinteractor_r))
  (:Released
    (Default|PickupReleased _bpc_worldinteractor_r)
    (Default|DragStop _bpc_worldinteractor_r)))

(event Input|KeyboardEvents|MotionControllerLeftThumbstick
  (params (Key :type Key%20Structure :default "None"))
  (bind _bp_traceinteractor_l (Variables|Default|GetBP_TraceInteractor_L))
  ;[1 1 1] Activate trace
  (:Pressed
    (Default|ActivateEventDown _bp_traceinteractor_l))
  (:Released
    (Default|ActivateEventUp _bp_traceinteractor_l)))

(event Input|KeyboardEvents|MotionControllerRightThumbstick
  (params (Key :type Key%20Structure :default "None"))
  (bind _bp_traceinteractor_r (Variables|Default|GetBP_TraceInteractor_R))
  (:Pressed
    (Default|ActivateEventDown _bp_traceinteractor_r))
  (:Released
    (Default|ActivateEventUp _bp_traceinteractor_r)))

(event Input|KeyboardEvents|MotionControllerLeftTrigger
  (params (Key :type Key%20Structure :default "None"))
  (bind _bpc_worldinteractor_l (Variables|Default|GetBPC_WorldInteractor_L))
  ;[1 1 1] Use objects
  (:Pressed
    (Default|UsePressed _bpc_worldinteractor_l))
  (:Released
    (Default|UseReleased _bpc_worldinteractor_l)))

(event Input|KeyboardEvents|MotionControllerRightTrigger
  (params (Key :type Key%20Structure :default "None"))
  (bind _bpc_worldinteractor_r (Variables|Default|GetBPC_WorldInteractor_R))
  ;[1 1 1] Use objects
  (:Pressed
    (Default|UsePressed _bpc_worldinteractor_r))
  (:Released
    (Default|UseReleased _bpc_worldinteractor_r)))

(fn ConstructionScript)