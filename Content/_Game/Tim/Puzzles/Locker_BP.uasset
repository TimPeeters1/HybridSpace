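; Locker puzzle actor whose door swings open when a designated key object overlaps its trigger box.
; The overlap, gated by a HasOpened flag that this graph never sets, plays a timeline that drives the door's yaw.
; A Key component starts hidden, and a DoOnce on the timeline's update sets it visible then immediately hidden again.
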(event OnComponentBeginOverlap(Box)
  (params (OverlappedComponent :type Primitive%20Component%20Object%20Reference) (OtherActor :type Actor%20Object%20Reference) (OtherComp :type Primitive%20Component%20Object%20Reference) (OtherBodyIndex :type Integer) (bFromSweep :type Boolean) (SweepResult :type Hit%20Result%20Structure%20%28by%20ref%29))
  (if (== OtherActor (Variables|Default|GetKeyObject))
    (if (not (Variables|Default|GetHasOpened))
      (bind _rotation (Timeline|Timeline_0 Play)
        (:Update
          (Transformation|SetRelativeRotation (Variables|Default|GetLocker_Door__2_) (Math|Rotator|MakeRotator 0.0 0.0 (.Z (Math|Vector|BreakVector (Math|Vector|MakeVector 0.0 0.0 _rotation)))) false false)
          (Utilities|FlowControl|DoOnce false
            (:Completed
              (Rendering|SetVisibility (Variables|Default|GetKey) true false)
              (Rendering|SetVisibility (Variables|Default|GetKey) false false))))))))

(event EventBeginPlay
  (Rendering|SetVisibility (Variables|Default|GetKey) false false))

(fn ConstructionScript)