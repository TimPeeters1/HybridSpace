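; Puzzle drawer actor that hides a referenced key object at start and reveals it when opened.
; On BeginPlay the key is made invisible, with gravity and collision disabled.
; OpenDrawer restores all three, plays an open sound at the drawer's location and runs a timeline to move the drawer mesh.
; The timeline's Location output is added as a relative offset on every update, so movement accumulates rather than interpolating between fixed positions.
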(event Custom|OpenDrawer
  (bind _keyobject (Variables|Default|GetKeyObject))
  (bind _staticmeshcomponent (Variables|/Script/Engine.StaticMeshActor|GetStaticMeshComponent _keyobject))
  (Rendering|SetVisibility (Variables|/Script/Engine.Actor|GetRootComponent _keyobject) true false)
  (Collision|SetCollisionEnabled _staticmeshcomponent "QueryAndPhysics")
  (Physics|SetEnableGravity _staticmeshcomponent true)
  (Audio|PlaySoundatLocation (Variables|Default|GetOpenSound) (Transformation|GetActorLocation self) "0, 0, 0" 1.0 1.0 0.0 0 0 0)
  (bind _location (Timeline|Timeline_0 Play)
    (:Update
      (Transformation|AddRelativeLocation (Variables|Debug|GetStaticMeshComponent) _location false false))))

(event EventBeginPlay
  (bind _keyobject (Variables|Default|GetKeyObject))
  (bind _staticmeshcomponent (Variables|/Script/Engine.StaticMeshActor|GetStaticMeshComponent _keyobject))
  (Rendering|SetVisibility (Variables|/Script/Engine.Actor|GetRootComponent (Variables|Default|GetKeyObject)) false false)
  (Physics|SetEnableGravity _staticmeshcomponent false)
  (Collision|SetCollisionEnabled _staticmeshcomponent "NoCollision"))

(fn ConstructionScript)