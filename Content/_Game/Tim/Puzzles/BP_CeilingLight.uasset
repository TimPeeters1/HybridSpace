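; BP_CeilingLight is a ceiling light actor whose two lights flicker randomly.
; Tick runs a Delay of random length between MinDelay and MaxDelay, then sets Light1 and Light2 to a random intensity between MinIntensity and MaxIntensity.
; Because the pending Delay ignores repeat Tick calls, it acts as an irregular flicker timer.
; BeginPlay stores the static mesh component in a variable that this graph never reads.
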(event EventTick
  (params (DeltaSeconds :type Float%20%28single-precision%29))
  (Utilities|FlowControl|Delay (Math|Random|RandomFloatinRange (Variables|Default|GetMinDelay) (Variables|Default|GetMaxDelay)))
  (Rendering|Components|Light|SetIntensity (Variables|Default|GetLight2) (Math|Random|RandomFloatinRange (Variables|Default|GetMinIntensity) (Variables|Default|GetMaxIntensity))))

(event EventBeginPlay
  (Variables|Default|SetStaticMesh (Variables|Debug|GetStaticMeshComponent)))

(fn ConstructionScript)