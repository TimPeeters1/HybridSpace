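; Puzzle ceiling light with two light components and an emissive-style on/off material swap, driven by a linked LightButton's LightIsOn state.
; While on, Tick uses randomized Delays to cycle both lights between high and low intensity ranges, swapping the mesh material with them.
; FlickerAllLights and ResetAllLights swap flicker and normal timing/intensity presets.
; TurnOffAllLights hides both lights and clears the button's LightIsOn.
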(event EventTick
  (params (DeltaSeconds :type Float%20%28single-precision%29))
  (if (Variables|/Game/_Game/Tim/Puzzles/LightButton1.LightButton1_C|GetlightIsOn (Variables|Default|GetLightButton))
    (Utilities|FlowControl|Delay (Math|Random|RandomFloatinRange (Variables|Default|GetMinFirstDelay) (Variables|Default|GetMaxFirstDelay)))
    (Rendering|Material|SetMaterial (Variables|Debug|GetStaticMeshComponent) 2 (Variables|Default|GetLightON))
    (Rendering|Components|Light|SetIntensity (Variables|Default|GetLight2) (Math|Random|RandomFloatinRange (Variables|Default|GetMinHIGHIntensity) (Variables|Default|GetMaxHIGHIntensity)))
    (Utilities|FlowControl|Delay (Math|Random|RandomFloatinRange (Variables|Default|GetMinSecondDelay) (Variables|Default|GetMaxSecondDelay)))
    (Rendering|Components|Light|SetIntensity (Variables|Default|GetLight1) (Math|Random|RandomFloatinRange (Variables|Default|GetMinLOWIntensity) (Variables|Default|GetMaxLOWIntensity)))
    (Rendering|Material|SetMaterial (Variables|Debug|GetStaticMeshComponent) 2 (Variables|Default|GetLightOFF))))

(event EventBeginPlay
  (Variables|Default|SetStaticMesh (Variables|Debug|GetStaticMeshComponent)))

(fn ConstructionScript)

(fn FlickerAllLights
  (Variables|Default|SetisFlickering true)
  (Variables|Default|SetMinFirstDelay (Variables|Default|GetMinFirstDelay_F))
  (Variables|Default|SetMaxFirstDelay (Variables|Default|GetMaxFirstDelay_F))
  (Variables|Default|SetMinHIGHIntensity (Variables|Default|GetMinHIGHIntensity_F))
  (Variables|Default|SetMaxHIGHIntensity (Variables|Default|GetMaxHIGHIntensity_F))
  (Variables|Default|SetMinSecondDelay (Variables|Default|GetMinSecondDelay_F))
  (Variables|Default|SetMaxSecondDelay (Variables|Default|GetMaxSecondDelay_F))
  (Variables|Default|SetMinLOWIntensity (Variables|Default|GetMinLOWIntensity_F))
  (Variables|Default|SetMaxLOWIntensity (Variables|Default|GetMaxLOWIntensity_F))
  (Development|PrintString "flickering"))

(fn ResetAllLights
  (Variables|Default|SetisFlickering false)
  (Variables|Default|SetMinFirstDelay (Variables|Default|GetMinFirstDelay_N))
  (Variables|Default|SetMaxFirstDelay (Variables|Default|GetMaxFirstDelay_N))
  (Variables|Default|SetMinHIGHIntensity (Variables|Default|GetMinHIGHIntensity_N))
  (Variables|Default|SetMaxHIGHIntensity (Variables|Default|GetMaxHIGHIntensity_N))
  (Variables|Default|SetMinSecondDelay (Variables|Default|GetMinSecondDelay_N))
  (Variables|Default|SetMaxSecondDelay (Variables|Default|GetMaxSecondDelay_N))
  (Variables|Default|SetMinLOWIntensity (Variables|Default|GetMinLOWIntensity_N))
  (Variables|Default|SetMaxLOWIntensity (Variables|Default|GetMaxLOWIntensity_N))
  (Development|PrintString "back to basic"))

(fn TurnOffAllLights
  (Rendering|SetVisibility (Variables|Default|GetLight1) false false)
  (Rendering|SetVisibility (Variables|Default|GetLight2) false false)
  (Variables|/Game/_Game/Tim/Puzzles/LightButton1.LightButton1_C|SetlightIsOn (Variables|Default|GetLightButton) false))